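; Rotating-stone puzzle actor: the player enters a box to switch to its camera with mouse clicking and a UI widget, and leaves to restore the character view.
; BeginPlay spawns a row of five randomly rotated stone meshes, mapping each component to an index.
; Clicks turn stones in quarter steps tracked in CurrentSide.
; The check button compares that array with the answer, changing material permanently on success or briefly on failure.
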(event OnComponentBeginOverlap(Box)
  (params (OverlappedComponent :type Primitive%20Component%20Object%20Reference) (OtherActor :type Actor%20Object%20Reference) (OtherComp :type Primitive%20Component%20Object%20Reference) (OtherBodyIndex :type Integer) (bFromSweep :type Boolean) (SweepResult :type Hit%20Result%20Structure%20%28by%20ref%29))
  (bind _returnvalue (Game|GetPlayerController 0))
  ;[1 1 1] Change View To Stone Camera
  (if bFromSweep
    (Game|Player|SetViewTargetwithBlend (Game|GetPlayerController 0) self 1.0 "VTBlend_Linear" 0.0 false)
    (Variables|/Script/Engine.PlayerController|SetbShowMouseCursor _returnvalue true)
    (Variables|/Script/Engine.PlayerController|SetbEnableClickEvents _returnvalue true)
    (bind _returnvalue_2 (UserInterface|CreateWidget "/Game/BluePrint/Tutorial/BluePrints/WD_TStone2.WD_TStone2_C" (Game|GetPlayerController 0)))
    (UserInterface|Viewport|AddtoViewport _returnvalue_2 0)))

(event OnComponentEndOverlap(Box)
  (params (OverlappedComponent :type Primitive%20Component%20Object%20Reference) (OtherActor :type Actor%20Object%20Reference) (OtherComp :type Primitive%20Component%20Object%20Reference) (OtherBodyIndex :type Integer))
  (bind _returnvalue (Game|GetPlayerController 0))
  ;[1 1 1] Change View To Stone Camera
  (bind _asbp_third_person_character (Utilities|Casting|CastToBP_ThirdPersonCharacter OtherActor))
  (Game|Player|SetViewTargetwithBlend (Game|GetPlayerController 0) _asbp_third_person_character 0.5 "VTBlend_Linear" 0.0 false)
  (Variables|/Script/Engine.PlayerController|SetbShowMouseCursor _returnvalue false)
  (Variables|/Script/Engine.PlayerController|SetbEnableClickEvents _returnvalue false))

(event Custom|Click%20-%20Check
  (params (TouchedComponent :type Primitive%20Component%20Object%20Reference) (ButtonPressed :type Key%20Structure :default "None"))
  ;[1 1 1] Check - Logic
  (if (Variables|Default|GetIsOpened)
    (if (Utilities|Array|Identical (Variables|Default|GetCorrect) (Variables|Default|GetCurrentSide))
      (Rendering|Material|SetMaterial TouchedComponent 0 "/Game/BluePrint/StonePuzzle2/MESHES/Material_001.Material_001")
      (Variables|Default|SetIsOpened false)
      (else
        (Rendering|Material|SetMaterial TouchedComponent 0 "/Game/BluePrint/StonePuzzle2/MESHES/Material_001.Material_001")
        (Utilities|FlowControl|Delay 0.7)
        (Rendering|Material|SetMaterial TouchedComponent 0 "/Game/BluePrint/StonePuzzle2/MESHES/Material_004.Material_004")))))

(event Custom|Click-Rotate
  (params (TouchedComponent :type Primitive%20Component%20Object%20Reference) (ButtonPressed :type Key%20Structure :default "None"))
  (bind _currentside (Variables|Default|GetCurrentSide))
  (bind _indexes (Variables|Default|GetIndexes))
  (bind (_value _returnvalue) (Utilities|Map|Find _indexes TouchedComponent))
  ;[1 1 1] Click - Rotate Mechanic
  (bind _result (Math|Integer|IncrementInt (Utilities|Array|Get(acopy) _currentside _value))
    (:%20%20
      (Utilities|Array|SetArrayElem _currentside _value (Math|Integer|%(Integer) _result 4) _returnvalue)
      (Transformation|AddLocalRotation TouchedComponent "0.000000,90.000000,0.000000" false false))))

(event EventBeginPlay
  ;[1 1 1] StonesGeneration
  (for _index (range 0 4)
    (bind _output_get (Variables|Default|SetRandomLocation (Math|Random|RandomInteger 3)))
    (bind _returnvalue (AddComponent|AddStaticMeshComponent false (Math|Transform|MakeTransform (+ (Math|Vector|MakeVector (Math|Conversions|ToFloat(Integer) (* _index 75)) 0.0 0.0) "0.000000,0.000000,-50.000000") (Math|Rotator|MakeRotator 0.0 0.0 (Math|Float|%(Float) (+ (* 9e+01 (Math|Conversions|ToFloat(Integer) _output_get)) 3.6e+02) 3.6e+02)) "25.000000,25.000000,25.000000")))
    (Utilities|Map|Add (Variables|Default|GetIndexes) _returnvalue _index)
    (EventDispatchers|AssignOnClicked _returnvalue (delegate Custom|Click-Rotate))
    (EventDispatchers|AssignOnClicked (Variables|Default|GetCheckButton) (delegate Custom|Click%20-%20Check))
    (Components|StaticMesh|SetStaticMesh _returnvalue "/Game/LevelObject/Cube_002.Cube_002")
    (Utilities|Array|SetArrayElem (Variables|Default|GetCurrentSide) (.Value (Utilities|Map|Find (Variables|Default|GetIndexes) _returnvalue)) _output_get (.ReturnValue (Utilities|Map|Find (Variables|Default|GetIndexes) _returnvalue)))
    (Utilities|Array|SetArrayElem (Variables|Default|GetCorrect) (.Value (Utilities|Map|Find (Variables|Default|GetIndexes) _returnvalue)) (Utilities|Array|Get(acopy) (Variables|Default|GetCorrectFR) (.Value (Utilities|Map|Find (Variables|Default|GetIndexes) _returnvalue))))))

(event Collision|EventActorBeginOverlap
  (params (OtherActor :type Actor%20Object%20Reference)))

(event EventTick
  (params (DeltaSeconds :type Float%20%28single-precision%29)))

(fn ConstructionScript)

(fn NewFunction
  (params (NewParam :type Boolean)))
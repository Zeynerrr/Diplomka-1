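; BP_StoneGeneration is an actor that builds a small upright wall of scaled-down cube meshes.
; The construction script uses nested loops to add a static mesh component per cell, spacing columns along X and rows along Z.
; An Interact event runs into a DoOnce with nothing after it, so interaction currently has no effect.
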(event Custom|Interact
  (params (Hit%20component :type Actor%20Component%20Object%20Reference))
  (Utilities|FlowControl|DoOnce false))

(event EventBeginPlay)

(event Collision|EventActorBeginOverlap
  (params (OtherActor :type Actor%20Object%20Reference)))

(event EventTick
  (params (DeltaSeconds :type Float%20%28single-precision%29)))

(fn ConstructionScript
  ;[1 1 1] Stone Generate
  (for _index (range 0 2)
    (for _index_2 (range 0 4)
      (bind _returnvalue (AddComponent|AddStaticMeshComponent false (Math|Transform|MakeTransform (Math|Vector|MakeVector (Math|Conversions|ToFloat(Integer) (* _index_2 25)) 0.0 (Math|Conversions|ToFloat(Integer) (* _index 30))) "0, 0, 0" "0.200000,0.200000,0.200000")))
      (Components|StaticMesh|SetStaticMesh _returnvalue "/Game/BluePrint/StoneGeneration/MESHES/box_Cube_001.box_Cube_001"))))
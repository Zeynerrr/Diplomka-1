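; Stone combination puzzle board: the player clicks stones and confirms with a check button to set it open.
; Construction script builds a Rows by Columns mesh grid; BeginPlay binds clicks and marks answers from CorrectCombination grid positions.
; Clicks light up to three stones; the button resets materials and compares selected against correct stones.
; Box overlap blends the view to the board and enables cursor clicking, restoring the character view on exit.
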(event OnComponentBeginOverlap(Box)
  (params (OverlappedComponent :type Primitive%20Component%20Object%20Reference) (OtherActor :type Actor%20Object%20Reference) (OtherComp :type Primitive%20Component%20Object%20Reference) (OtherBodyIndex :type Integer) (bFromSweep :type Boolean) (SweepResult :type Hit%20Result%20Structure%20%28by%20ref%29))
  (bind _returnvalue (Game|GetPlayerController 0))
  ;[1 1 1] Change View Stone Camera
  (if bFromSweep
    (Game|Player|SetViewTargetwithBlend (Game|GetPlayerController 0) self 1.0 "VTBlend_Linear" 0.0 false)
    (Variables|/Script/Engine.PlayerController|SetbShowMouseCursor _returnvalue true)
    (Variables|/Script/Engine.PlayerController|SetbEnableClickEvents _returnvalue true)))

(event OnComponentEndOverlap(Box)
  (params (OverlappedComponent :type Primitive%20Component%20Object%20Reference) (OtherActor :type Actor%20Object%20Reference) (OtherComp :type Primitive%20Component%20Object%20Reference) (OtherBodyIndex :type Integer))
  (bind _returnvalue (Game|GetPlayerController 0))
  ;[1 1 1] Change View Stone Camera
  (bind _asbp_third_person_character (Utilities|Casting|CastToBP_ThirdPersonCharacter OtherActor))
  (Game|Player|SetViewTargetwithBlend (Game|GetPlayerController 0) _asbp_third_person_character 0.5 "VTBlend_Linear" 0.0 false)
  (Variables|/Script/Engine.PlayerController|SetbShowMouseCursor _returnvalue false)
  (Variables|/Script/Engine.PlayerController|SetbEnableClickEvents _returnvalue false))

(event Custom|ClickComponent
  (params (TouchedComponent :type Primitive%20Component%20Object%20Reference) (ButtonPressed :type Key%20Structure :default "None"))
  ;[1 1 1] StoneVerification
  (if (< (Variables|Default|GetCheker) 3)
    (if (not (Variables|Default|Getis%20open))
      (Rendering|Material|SetMaterial TouchedComponent 0 "/Game/LevelObject/Materials/NeonMaterialInstance.NeonMaterialInstance")
      (Utilities|Set|Add (Variables|Default|Getselected) TouchedComponent)
      (Math|Integer|IncrementInt (Variables|Default|GetCheker)))))

(event Custom|ClickCheckButton
  (params (TouchedComponent :type Primitive%20Component%20Object%20Reference) (ButtonPressed :type Key%20Structure :default "None"))
  (bind _selected (Variables|Default|Getselected))
  ;[1 1 1] StoneVerification
  (if (not (Variables|Default|Getis%20open))
    (bind _result (Utilities|Set|ToArray _selected))
    (for _array_element _result
      (bind _asprimitive_component (Utilities|Casting|CastToPrimitiveComponent _array_element))
      (Rendering|Material|SetMaterial _asprimitive_component 0 "/Game/LevelObject/Materials/StoneMaterial.StoneMaterial")
      (Variables|Default|SetCheker 0))
    (if (== (Utilities|Set|Length _selected) (Utilities|Set|Length (Variables|Default|GetCorrect%20Components)))
      (bind _result_2 (Utilities|Set|ToArray _selected))
      (bind _array_element_2 (Utilities|Array|ForEachLoopwithBreak _result_2 :!label _label)
        (:LoopBody
          (if (not (Utilities|Set|Contains (Variables|Default|GetCorrect%20Components) _array_element_2))
            (Utilities|Set|Clear (Variables|Default|Getselected))
            (Variables|Default|Setis%20correct false)
            (goto _label Break)))
        (:Completed
          (if (Variables|Default|Getis%20correct)
            (Variables|Default|Setis%20open true)
            (else
              (Variables|Default|Setis%20correct false)))))
      (else
        (Utilities|Set|Clear (Variables|Default|Getselected))))
    (else
      (Variables|Default|SetCheker 0))))

(event EventBeginPlay
  (bind _columns (Variables|Default|GetColumns))
  ;[1 1 1] Stone Generation
  (for (_array_element _array_index) (Variables|Default|GetAll%20buttons)
    (EventDispatchers|BindEventtoOnClicked _array_element (delegate Custom|ClickComponent))
    (if (Utilities|Set|Contains (Variables|Default|GetCorrect%20combination) (Utilities|Struct|MakeS_pos (Math|Integer|%(Integer) _array_index _columns) (/ _array_index _columns)))
      (Utilities|Set|Add (Variables|Default|GetCorrect%20components) _array_element)))
  (EventDispatchers|BindEventtoOnClicked (Variables|Default|GetButton) (delegate Custom|ClickCheckButton)))

(fn ConstructionScript
  (Utilities|FlowControl|Sequence
    (:then_0
      (for _index (range 0 (- (Variables|Default|GetRows) 1))
        (for _index_2 (range 0 (- (Variables|Default|GetColumns) 1))
          (bind _returnvalue (AddComponent|AddStaticMeshComponent false (Math|Transform|MakeTransform (+ (Math|Vector|MakeVector (Math|Conversions|ToFloat(Integer) (* _index_2 100)) 0.0 (Math|Conversions|ToFloat(Integer) (* _index -90))) (Math|Vector|MakeVector 335.0 0.0 1e+02)) "0, 0, 0" "0.700000,0.700000,0.700000")))
          (Utilities|Array|Add (Variables|Default|GetAll%20buttons) _returnvalue))))))
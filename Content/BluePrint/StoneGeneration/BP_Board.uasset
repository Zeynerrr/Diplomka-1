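; BP_Board is a stone-combination puzzle that switches to its own view with mouse clicking on overlap, returning to the character's view on exit.
; BeginPlay builds a grid of clickable meshes, sorting them against CorrectCombination into correct and other components.
; Clicking highlights and records up to three stones.
; Clicking the Cube restores their materials and validates the selection, setting IsOpen on a match, which locks further selection.
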(event OnComponentBeginOverlap(r)
  (params (OverlappedComponent :type Primitive%20Component%20Object%20Reference) (OtherActor :type Actor%20Object%20Reference) (OtherComp :type Primitive%20Component%20Object%20Reference) (OtherBodyIndex :type Integer) (bFromSweep :type Boolean) (SweepResult :type Hit%20Result%20Structure%20%28by%20ref%29))
  (bind _returnvalue (Game|GetPlayerController 0))
  ;[1 1 1] Change View Stone Camera
  (if bFromSweep
    (Game|Player|SetViewTargetwithBlend (Game|GetPlayerController 0) self 1.0 "VTBlend_Linear" 0.0 false)
    (Variables|/Script/Engine.PlayerController|SetbShowMouseCursor _returnvalue true)
    (Variables|/Script/Engine.PlayerController|SetbEnableClickEvents _returnvalue true)))

(event OnComponentEndOverlap(r)
  (params (OverlappedComponent :type Primitive%20Component%20Object%20Reference) (OtherActor :type Actor%20Object%20Reference) (OtherComp :type Primitive%20Component%20Object%20Reference) (OtherBodyIndex :type Integer))
  (bind _returnvalue (Game|GetPlayerController 0))
  ;[1 1 1] Change View Stone Camera
  (bind _asbp_third_person_character (Utilities|Casting|CastToBP_ThirdPersonCharacter OtherActor))
  (Game|Player|SetViewTargetwithBlend (Game|GetPlayerController 0) _asbp_third_person_character 0.5 "VTBlend_Linear" 0.0 false)
  (Variables|/Script/Engine.PlayerController|SetbShowMouseCursor _returnvalue false)
  (Variables|/Script/Engine.PlayerController|SetbEnableClickEvents _returnvalue false))

(event Custom|OnClicked_Event
  (params (TouchedComponent :type Primitive%20Component%20Object%20Reference) (ButtonPressed :type Key%20Structure :default "None"))
  ;[1 1 1] StoneVerification
  (if (< (Variables|Default|GetChecker) 3)
    (if (not (Variables|Default|GetIsOpen))
      (Rendering|Material|SetMaterial TouchedComponent 0 "/Game/LevelObject/Materials/NeonMaterialInstance.NeonMaterialInstance")
      (Utilities|Set|Add (Variables|Default|GetSelected) TouchedComponent)
      (Math|Integer|IncrementInt (Variables|Default|GetChecker)))))

(event Custom|OnClickedCheck
  (params (TouchedComponent :type Primitive%20Component%20Object%20Reference) (ButtonPressed :type Key%20Structure :default "None"))
  (bind _selected (Variables|Default|GetSelected))
  ;[1 1 1] StoneVerification
  (if (not (Variables|Default|GetIsOpen))
    (bind _result (Utilities|Set|ToArray _selected))
    (for _array_element _result
      (bind _asprimitive_component (Utilities|Casting|CastToPrimitiveComponent _array_element))
      (Rendering|Material|SetMaterial _asprimitive_component 0 "/Game/LevelObject/Materials/StoneMaterial.StoneMaterial")
      (Variables|Default|SetChecker 0))
    (if (== (Utilities|Set|Length _selected) (Utilities|Set|Length (Variables|Default|GetCorrect%20Components)))
      (bind _result_2 (Utilities|Set|ToArray _selected))
      (bind _array_element_2 (Utilities|Array|ForEachLoopwithBreak _result_2 :!label _label)
        (:LoopBody
          (if (not (Utilities|Set|Contains (Variables|Default|GetCorrect%20Components) _array_element_2))
            (Utilities|Set|Clear (Variables|Default|GetSelected))
            (Variables|Default|SetIsCorrect false)
            (goto _label Break)))
        (:Completed
          (if (Variables|Default|GetIsCorrect)
            (Variables|Default|SetIsOpen true)
            (else
              (Variables|Default|SetIsCorrect true)))))
      (else
        (Utilities|Set|Clear (Variables|Default|GetSelected))))
    (else
      (Variables|Default|SetChecker 0))))

(event Collision|EventActorBeginOverlap
  (params (OtherActor :type Actor%20Object%20Reference)))

(event EventBeginPlay
  ;[1 1 1] Stone Generation
  (for _index (range 0 2)
    (for _index_2 (range 0 4)
      (bind _returnvalue (AddComponent|AddStaticMeshComponent false (Math|Transform|MakeTransform (+ (Math|Vector|MakeVector (Math|Conversions|ToFloat(Integer) (* _index_2 100)) (Math|Conversions|ToFloat(Integer) (* _index -90)) 0.0) "335.000000,0.000000,200.000000") "0, 0, 0" "0.200000,0.200000,0.200000")))
      (EventDispatchers|AssignOnClicked _returnvalue (delegate Custom|OnClicked_Event))
      (EventDispatchers|BindEventtoOnClicked (Variables|Default|GetCube) (delegate Custom|OnClickedCheck))
      (Components|StaticMesh|SetStaticMesh _returnvalue "/Game/LevelObject/NeonCube.NeonCube")
      (if (Utilities|Set|Contains (Variables|Default|GetCorrect%20Combination) (Utilities|Struct|MakeS_pos _index _index_2))
        (Utilities|Set|Add (Variables|Default|GetCorrect%20Components) _returnvalue)
        (else
          (Utilities|Set|Add (Variables|Default|GetOther%20Components) _returnvalue))))))

(fn ConstructionScript)
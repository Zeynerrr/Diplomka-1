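; BP_TRAP1 is a trap that drains the player character's HP while its Box is overlapped.
; Box begin and end overlap events toggle a Check flag for any actor, without filtering.
; Tick, gated by Check and the overlap event's FromSweep value, runs a 0.4-second Delay, then applies -10 through UpdateHp on player 0's BP_ThirdPersonCharacter, producing repeated damage.
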(event OnComponentBeginOverlap(Box)
  (params (OverlappedComponent :type Primitive%20Component%20Object%20Reference) (OtherActor :type Actor%20Object%20Reference) (OtherComp :type Primitive%20Component%20Object%20Reference) (OtherBodyIndex :type Integer) (bFromSweep :type Boolean) (SweepResult :type Hit%20Result%20Structure%20%28by%20ref%29))
  (Variables|Default|SetCheck true))

(event OnComponentEndOverlap(Box)
  (params (OverlappedComponent :type Primitive%20Component%20Object%20Reference) (OtherActor :type Actor%20Object%20Reference) (OtherComp :type Primitive%20Component%20Object%20Reference) (OtherBodyIndex :type Integer))
  (Variables|Default|SetCheck false))

(event EventBeginPlay)

(event Collision|EventActorBeginOverlap
  (params (OtherActor :type Actor%20Object%20Reference)))

(event EventTick
  (params (DeltaSeconds :type Float%20%28single-precision%29))
  (if (stale OnComponentBeginOverlap(Box) bFromSweep)
    (if (Variables|Default|GetCheck)
      (Utilities|FlowControl|Delay 0.4)
      (bind _asbp_third_person_character (Utilities|Casting|CastToBP_ThirdPersonCharacter (Game|GetPlayerCharacter 0)))
      (Default|UpdateHp _asbp_third_person_character -1e+01))))

(fn ConstructionScript)